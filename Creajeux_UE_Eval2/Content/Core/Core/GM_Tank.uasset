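; GM_Tank is the tank game's game mode, handling the start countdown and the win condition.
; BeginPlay creates the WB_HUDGame widget and disables player input until a looping one-second timer counts down to "GO!!!".
; Tick polls for BP_Turret actors and, once none remain, disables input and adds a fresh HUD showing the win element, repeating every frame with no guard.
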(event `self.ReceiveBeginPlay`
  (bind _returnvalue (`|CreateWidget` "/Game/Core/Blueprint/WB_HUDGame.WB_HUDGame_C"))
  (bind _output_get (set `self.CountdownWidget` _returnvalue))
  (`UserWidget.AddToViewport` _output_get 0)
  (`Widget.SetVisibility` (`/Game/Core/Blueprint/WB_HUDGame.Lost` (`self.CountdownWidget`)) "Hidden")
  (`Widget.SetVisibility` (`/Game/Core/Blueprint/WB_HUDGame.Win` (`self.CountdownWidget`)) "Hidden")
  (bind _returnvalue_2 (`KismetSystemLibrary.K2_SetTimerDelegate` (delegate `Take Countdown`) 1.0 true))
  (`self.DisableInput` (`GameplayStatics.GetPlayerPawn` 0) (`GameplayStatics.GetPlayerController` 0)))

(event `Take Countdown`
  (`/Engine/EditorBlueprintResources/StandardMacros.DecrementInt` (`self.Count`)
    (:`  `
      (`TextBlock.SetText` (`/Game/Core/Blueprint/WB_HUDGame.Countdown` (`self.CountdownWidget`)) (`KismetTextLibrary.Conv_IntToText` (`self.Count`)))
      (if (<= (`self.Count`) 0)
        (`KismetSystemLibrary.K2_ClearAndInvalidateTimerHandle` (stale `self.ReceiveBeginPlay` _returnvalue_2))
        (`TextBlock.SetText` (`/Game/Core/Blueprint/WB_HUDGame.Countdown` (`self.CountdownWidget`)) "GO!!!")
        (`self.EnableInput` (`GameplayStatics.GetPlayerPawn` 0) (`GameplayStatics.GetPlayerController` 0))
        (`KismetSystemLibrary.Delay` 1.0)
        (`Widget.RemoveFromParent` (`/Game/Core/Blueprint/WB_HUDGame.Countdown` (`self.CountdownWidget`)))))))

(event `self.ReceiveTick`
  (params (DeltaSeconds :type "Float (single-precision)"))
  (bind _outactors (`GameplayStatics.GetAllActorsOfClass` "/Game/Core/Blueprint/BP_Turret.BP_Turret_C"))
  (if (<= (`KismetArrayLibrary.Array_Length` _outactors) 0)
    (`self.DisableInput` (`GameplayStatics.GetPlayerPawn` 0) (`GameplayStatics.GetPlayerController` 0))
    (bind _returnvalue (`|CreateWidget` "/Game/Core/Blueprint/WB_HUDGame.WB_HUDGame_C"))
    (bind _output_get (set `self.CountdownWidget` _returnvalue))
    (`UserWidget.AddToViewport` _output_get 0)
    (`Widget.SetVisibility` (`/Game/Core/Blueprint/WB_HUDGame.Lost` (`self.CountdownWidget`)) "Hidden")
    (`Widget.SetVisibility` (`/Game/Core/Blueprint/WB_HUDGame.Countdown` (`self.CountdownWidget`)) "Hidden")))

(fn `UserConstructionScript`)